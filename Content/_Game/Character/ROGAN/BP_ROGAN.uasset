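; BP_ROGAN is the Blueprint for the ROGAN character, with a follow camera and a motion warping component.
; The construction script constrains the follow camera's aspect ratio, and BeginPlay disables all root motion modifiers on the motion warping component.
; Unconnected leftover nodes for setting a warp target and printing directional input never run, and Tick is empty.
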(event `self.ReceiveBeginPlay`
  (`MotionWarpingComponent.DisableAllRootMotionModifiers` (`self.MotionWarpingComponent`)))

(event `self.ReceiveTick`
  (params (DeltaSeconds :type "Float (single-precision)")))

(fn `UserConstructionScript`
  (set `CameraComponent.bConstrainAspectRatio` true (`self.FollowCamera`)))