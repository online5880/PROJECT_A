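; BP_ROGAN is a character Blueprint that adds a ledge climb on the Q key.
; A forward trace finds a wall, then a vertical trace just past it finds the top and sets the "Climb" motion warp target.
; It switches to Flying, disables input and plays the 1m or 2m montage section by ledge height.
; When the montage ends, it restores walking and input and turns the character to face along the inverse wall normal.
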(event `self.ReceiveBeginPlay`)

(event `self.ReceiveTick`
  (params (DeltaSeconds :type "Float (single-precision)")))

(event `Key|Q`
  (params (Key :type "Key Structure"))
  (bind _returnvalue (`self.K2_GetActorLocation`))
  (bind (_returnvalue_x _returnvalue_y _returnvalue_z) (`KismetMathLibrary.BreakVector` (`self.K2_GetActorLocation`)))
  (bind _climb_montage (`self.Climb_Montage`))
  (bind _returnvalue_2 (`SkeletalMeshComponent.GetAnimInstance` (`self.Mesh`)))
  (:`Pressed`
    (bind (_outhit _returnvalue_3) (`KismetSystemLibrary.LineTraceSingleForObjects` :`Start` _returnvalue :`End` (+ _returnvalue (* (`self.GetActorForwardVector`) 125.0)) :`ObjectTypes` (`|MakeArray` "ObjectTypeQuery1" :!type "EObjectTypeQuery Enum") :`DrawDebugType` "ForDuration"))
    (if _returnvalue_3
      (bind (_bblockinghit _binitialoverlap _time _distance _location _impactpoint _normal) (`GameplayStatics.BreakHitResult` _outhit))
      (bind _returnvalue_4 (`KismetMathLibrary.MakeRotFromX` _normal))
      (bind _returnvalue_5 (+ _location (* (`KismetMathLibrary.GetForwardVector` _returnvalue_4) -50.0)))
      (bind (_outhit_2 _returnvalue_6) (`KismetSystemLibrary.LineTraceSingleForObjects` :`Start` (+ _returnvalue_5 (0.0 0.0 200.0)) :`End` (- _returnvalue_5 (0.0 0.0 200.0)) :`ObjectTypes` (`|MakeArray` "ObjectTypeQuery1" :!type "EObjectTypeQuery Enum") :`DrawDebugType` "ForDuration"))
      (if _returnvalue_6
        (bind (_bblockinghit_2 _binitialoverlap_2 _time_2 _distance_2 _location_2) (`GameplayStatics.BreakHitResult` _outhit_2))
        (bind _returnvalue_7 (- (.z _location_2) _returnvalue_z))
        (`KismetSystemLibrary.PrintString` (`KismetStringLibrary.Conv_DoubleToString` _returnvalue_7))
        (`MotionWarpingComponent.AddOrUpdateWarpTargetFromLocationAndRotation` (`self.MotionWarpingComponent`) "Climb" _location_2 _returnvalue_4)
        (`CharacterMovementComponent.SetMovementMode` (`self.CharacterMovement`) "MOVE_Flying" 0)
        (`self.DisableInput` (`GameplayStatics.GetPlayerController` 0))
        ;[1 1 1] Comment
        (`AnimInstance.Montage_Play` _returnvalue_2 _climb_montage 1.0 "MontageLength" 0.0 true)
        (`AnimInstance.Montage_JumpToSection` _returnvalue_2 (select `int` (`KismetMathLibrary.SelectInt` 0 1 (> _returnvalue_7 100.0)) :`0` "Climb_2m" :`1` "Climb_1m" :!type "Name") _climb_montage)
        (add `AnimInstance.OnMontageEnded` _returnvalue_2 (delegate `CustomEvent`))))))

(event `CustomEvent`
  (params (Montage :type "AnimMontage Object Reference") (bInterrupted :type Boolean))
  (bind (_returnvalue_roll _returnvalue_pitch) (`KismetMathLibrary.BreakRotator` (`self.K2_GetActorRotation`)))
  (`CharacterMovementComponent.SetMovementMode` (`self.CharacterMovement`) "MOVE_Walking" 0)
  (`self.EnableInput` (`GameplayStatics.GetPlayerController` 0))
  (`self.K2_SetActorRotation` (`KismetMathLibrary.MakeRotator` _returnvalue_roll _returnvalue_pitch (+ (.yaw (`KismetMathLibrary.MakeRotFromX` (`.Normal` (`GameplayStatics.BreakHitResult` (stale `Key|Q` _outhit))))) 180.0))))

(fn `UserConstructionScript`
  (set `CameraComponent.bConstrainAspectRatio` true (`self.FollowCamera`)))